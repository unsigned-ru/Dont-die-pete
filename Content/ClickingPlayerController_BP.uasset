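; Player controller that turns jump and click input into actions for the Pete character.
; Jump input calls OnJump on the controlled Pete_BP pawn while AllowedToJump is true.
; On BeginPlay it binds to the PeteGameState death event, whose handler disables jumping.
; Click input calls LineTraceForClickableObject, which is not defined in this Blueprint, and is not gated by the jump flag.
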(event `self.ReceiveBeginPlay`
  (bind _aspete_game_state (cast `PeteGameState` (`GameplayStatics.GetGameState`)))
  (add `PeteGameState.onPeteDeath` _aspete_game_state (delegate `onPeteDeath`)))

(event `onPeteDeath`
  (set `self.AllowedToJump` false))

(event `InputAction|Jump`
  (params (Key :type "Key Structure"))
  (:`Pressed`
    (if (`self.AllowedToJump`)
      (bind _aspete_bp (cast `/Game/Pete_BP` (`self.K2_GetPawn`)))
      (`/Game/Pete_BP.OnJump` _aspete_bp))))

(event `InputAction|Click`
  (params (Key :type "Key Structure"))
  (:`Pressed`
    (`self.LineTraceForClickableObject`)))

(fn `UserConstructionScript`)